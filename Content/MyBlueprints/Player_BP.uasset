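; Pressable actor that changes color, moves vertically and plays a sound when its Box is overlapped.
; The PressEvent timeline drives a dynamic material's Color and the actor's absolute Z, reversing when the overlap ends.
; Timeline updates pick the sound from the actor's own display name (Player A or Player B).
; A SoundPlaying flag, cleared on end overlap, stops the sound retriggering every update.
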(event `self.ReceiveBeginPlay`
  (bind _returnvalue (`PrimitiveComponent.CreateDynamicMaterialInstance` (`self.StaticMesh`) 0 null "None"))
  (set `self.DynamicMaterialInstance` _returnvalue))

(event `self.Box.OnComponentBeginOverlap`
  (params (OverlappedComponent :type "PrimitiveComponent Object Reference") (OtherActor :type "Actor Object Reference") (OtherComp :type "PrimitiveComponent Object Reference") (OtherBodyIndex :type Integer) (bFromSweep :type Boolean) (SweepResult :type "HitResult Structure (by ref)"))
  (bind (_returnvalue_x _returnvalue_y) (`KismetMathLibrary.BreakVector` (`self.K2_GetActorLocation`)))
  (bind (_direction _downplay _red _green _blue) (`Timeline|PressEvent` :!label _label)
    (:`Update`
      (`MaterialInstanceDynamic.SetVectorParameterValue` (`self.DynamicMaterialInstance`) "Color" (`KismetMathLibrary.MakeColor` _red _green _blue))
      (`self.K2_SetActorLocation` (`KismetMathLibrary.MakeVector` _returnvalue_x _returnvalue_y _downplay))
      (switch `string` (`KismetSystemLibrary.GetDisplayName` (`ActorComponent.GetOwner` OverlappedComponent))
        (:`Player_A`
          (if (not (`self.soundPlaying`))
            (`GameplayStatics.PlaySoundAtLocation` "/Game/Audio/sound_a.sound_a" (0.0 0.0 0.0) (struct) 1.0 1.0 0.0 null null null)
            (set `self.soundPlaying` true)))
        (:`Player_B`
          (if (not (`self.soundPlaying`))
            (`GameplayStatics.PlaySoundAtLocation` "/Game/Audio/sound_b.sound_b" (0.0 0.0 0.0) (struct) 1.0 1.0 0.0 null null null)
            (set `self.soundPlaying` true)))))))

(event `self.Box.OnComponentEndOverlap`
  (params (OverlappedComponent :type "PrimitiveComponent Object Reference") (OtherActor :type "Actor Object Reference") (OtherComp :type "PrimitiveComponent Object Reference") (OtherBodyIndex :type Integer))
  (set `self.soundPlaying` false)
  (goto _label :!via `Reverse`))

(fn `UserConstructionScript`)