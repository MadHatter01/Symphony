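; BP_sylo_instrument is a xylophone-style instrument actor whose eight trigger boxes each play a musical note when overlapped.
; Overlapping its Widget component starts auto-play: after a short delay, it reads row "s1" of the SONGDATA table.
; A delayed custom loop steps through that row's Line1 notes, spawning a BP_soundball at the static mesh matching each note.
; When the loop completes, it destroys all soundballs.
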(event `self.Box.OnComponentBeginOverlap`
  (params (OverlappedComponent :type "PrimitiveComponent Object Reference") (OtherActor :type "Actor Object Reference") (OtherComp :type "PrimitiveComponent Object Reference") (OtherBodyIndex :type Integer) (bFromSweep :type Boolean) (SweepResult :type "HitResult Structure (by ref)"))
  (`GameplayStatics.PlaySound2D` "/Game/Audio/sound_c.sound_c" 1.0 1.0 0.0 null null))

(event `self.Box1.OnComponentBeginOverlap`
  (params (OverlappedComponent :type "PrimitiveComponent Object Reference") (OtherActor :type "Actor Object Reference") (OtherComp :type "PrimitiveComponent Object Reference") (OtherBodyIndex :type Integer) (bFromSweep :type Boolean) (SweepResult :type "HitResult Structure (by ref)"))
  (`GameplayStatics.PlaySound2D` "/Game/Audio/sound_d1.sound_d1" 1.0 1.0 0.0 null null))

(event `self.Box6.OnComponentBeginOverlap`
  (params (OverlappedComponent :type "PrimitiveComponent Object Reference") (OtherActor :type "Actor Object Reference") (OtherComp :type "PrimitiveComponent Object Reference") (OtherBodyIndex :type Integer) (bFromSweep :type Boolean) (SweepResult :type "HitResult Structure (by ref)"))
  (`GameplayStatics.PlaySound2D` "/Game/Audio/sound_b.sound_b" 1.0 1.0 0.0 null null))

(event `self.Box2.OnComponentBeginOverlap`
  (params (OverlappedComponent :type "PrimitiveComponent Object Reference") (OtherActor :type "Actor Object Reference") (OtherComp :type "PrimitiveComponent Object Reference") (OtherBodyIndex :type Integer) (bFromSweep :type Boolean) (SweepResult :type "HitResult Structure (by ref)"))
  (`GameplayStatics.PlaySound2D` "/Game/Audio/sound_e1.sound_e1" 1.0 1.0 0.0 null null))

(event `self.Box3.OnComponentBeginOverlap`
  (params (OverlappedComponent :type "PrimitiveComponent Object Reference") (OtherActor :type "Actor Object Reference") (OtherComp :type "PrimitiveComponent Object Reference") (OtherBodyIndex :type Integer) (bFromSweep :type Boolean) (SweepResult :type "HitResult Structure (by ref)"))
  (`GameplayStatics.PlaySound2D` "/Game/Audio/sound_f.sound_f" 1.0 1.0 0.0 null null))

(event `self.Box7.OnComponentBeginOverlap`
  (params (OverlappedComponent :type "PrimitiveComponent Object Reference") (OtherActor :type "Actor Object Reference") (OtherComp :type "PrimitiveComponent Object Reference") (OtherBodyIndex :type Integer) (bFromSweep :type Boolean) (SweepResult :type "HitResult Structure (by ref)"))
  (`GameplayStatics.PlaySound2D` "/Game/Audio/sound_c2.sound_c2" 1.0 1.0 0.0 null null))

(event `self.Box4.OnComponentBeginOverlap`
  (params (OverlappedComponent :type "PrimitiveComponent Object Reference") (OtherActor :type "Actor Object Reference") (OtherComp :type "PrimitiveComponent Object Reference") (OtherBodyIndex :type Integer) (bFromSweep :type Boolean) (SweepResult :type "HitResult Structure (by ref)"))
  (`GameplayStatics.PlaySound2D` "/Game/Audio/sound_g.sound_g" 1.0 1.0 0.0 null null))

(event `self.Box5.OnComponentBeginOverlap`
  (params (OverlappedComponent :type "PrimitiveComponent Object Reference") (OtherActor :type "Actor Object Reference") (OtherComp :type "PrimitiveComponent Object Reference") (OtherBodyIndex :type Integer) (bFromSweep :type Boolean) (SweepResult :type "HitResult Structure (by ref)"))
  (`GameplayStatics.PlaySound2D` "/Game/Audio/sound_a.sound_a" 1.0 1.0 0.0 null null))

(event `self.ReceiveBeginPlay`)

(event `self.Widget.OnComponentBeginOverlap`
  (params (OverlappedComponent :type "PrimitiveComponent Object Reference") (OtherActor :type "Actor Object Reference") (OtherComp :type "PrimitiveComponent Object Reference") (OtherBodyIndex :type Integer) (bFromSweep :type Boolean) (SweepResult :type "HitResult Structure (by ref)"))
  (`GameplayStatics.PlaySound2D` "/Engine/EditorSounds/Notifications/CompileSuccess.CompileSuccess" 1.0 1.0 0.0 null null)
  (`KismetSystemLibrary.Delay` 3.0)
  (bind _returnvalue (`|GetDataTableRow` "/Game/SONGDATA.SONGDATA" "s1")
    (:`then`
      (bind _array_element (`/Game/CustomLoop.CustomLoop` (`.Line1_9_800A439B4729FF439C9309AB1DE35C4C` (break `/Game/SongDatastructure` _returnvalue)) 1.5)
        (:`LoopBody`
          (switch `string` _array_element
            (:`C`
              (`|SpawnActorFromClass` "/Game/BP_soundball.BP_soundball_C" (`SceneComponent.K2_GetComponentToWorld` (`self.StaticMesh`)) "Undefined" "OverrideRootScale" null null))
            (:`D`
              (`|SpawnActorFromClass` "/Game/BP_soundball.BP_soundball_C" (`SceneComponent.K2_GetComponentToWorld` (`self.StaticMesh1`)) "Undefined" "OverrideRootScale" null null))
            (:`E`
              (`|SpawnActorFromClass` "/Game/BP_soundball.BP_soundball_C" (`SceneComponent.K2_GetComponentToWorld` (`self.StaticMesh2`)) "Undefined" "OverrideRootScale" null null))
            (:`F`
              (`|SpawnActorFromClass` "/Game/BP_soundball.BP_soundball_C" (`SceneComponent.K2_GetComponentToWorld` (`self.StaticMesh3`)) "Undefined" "OverrideRootScale" null null))
            (:`G`
              (`KismetSystemLibrary.Delay` 0.0)
              (`|SpawnActorFromClass` "/Game/BP_soundball.BP_soundball_C" (`SceneComponent.K2_GetComponentToWorld` (`self.StaticMesh4`)) "Undefined" "OverrideRootScale" null null))
            (:`A`
              (`KismetSystemLibrary.Delay` 0.0)
              (`|SpawnActorFromClass` "/Game/BP_soundball.BP_soundball_C" (`SceneComponent.K2_GetComponentToWorld` (`self.StaticMesh5`)) "Undefined" "OverrideRootScale" null null))
            (:`B`
              (`|SpawnActorFromClass` "/Game/BP_soundball.BP_soundball_C" (`SceneComponent.K2_GetComponentToWorld` (`self.StaticMesh6`)) "Undefined" "OverrideRootScale" null null))
            (:`C1`
              (`|SpawnActorFromClass` "/Game/BP_soundball.BP_soundball_C" (`SceneComponent.K2_GetComponentToWorld` (`self.StaticMesh7`)) "Undefined" "OverrideRootScale" null null))))
        (:`Completed`
          (`KismetSystemLibrary.PrintString` "Hello")
          (bind _outactors (`GameplayStatics.GetAllActorsOfClass` "/Game/BP_soundball.BP_soundball_C"))
          (for _array_element_2 _outactors
            (`self.K2_DestroyActor` _array_element_2)))))))

(fn `UserConstructionScript`)