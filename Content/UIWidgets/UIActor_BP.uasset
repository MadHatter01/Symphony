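; UIActor_BP is an in-world info actor that shows an instrument's name, description and history when its collision is overlapped.
; The overlap event switches on the actor's own display name to pick one of two hardcoded Instrument_dataTable rows.
; ExpandUIWidget writes that row into text render components and reveals the description.
; Music playback, widget creation and text spawning nodes are unconnected leftovers that never run.
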(event `self.ReceiveActorBeginOverlap`
  (params (OtherActor :type "Actor Object Reference")))

(event `self.ReceiveBeginPlay`)

(event `self.collision.OnComponentBeginOverlap`
  (params (OverlappedComponent :type "PrimitiveComponent Object Reference") (OtherActor :type "Actor Object Reference") (OtherComp :type "PrimitiveComponent Object Reference") (OtherBodyIndex :type Integer) (bFromSweep :type Boolean) (SweepResult :type "HitResult Structure (by ref)"))
  (switch `string` (`KismetSystemLibrary.GetDisplayName` (`ActorComponent.GetOwner` OverlappedComponent))
    (:`UIActor_BP`
      (set `self.actorvalue` "I0")
      (bind _returnvalue (`|GetDataTableRow` "/Game/Instrument_dataTable.Instrument_dataTable" "I0")
        (:`then`
          (`self.ExpandUIWidget` _returnvalue))))
    (:`UIActor_BP2`
      (bind _returnvalue_2 (`|GetDataTableRow` "/Game/Instrument_dataTable.Instrument_dataTable" "I1")
        (:`then`
          (`self.ExpandUIWidget` _returnvalue_2))))))

(fn `ExpandUIWidget`
  (params (Instrument_DataStructure :type "/Game/Instrument_DataStructure Structure (by ref)"))
  (bind (_instrumentname _instrumentdescription _instrumenthistory) (break `/Game/Instrument_DataStructure` Instrument_DataStructure))
  (`TextRenderComponent.K2_SetText` (`self.TextRender`) (`KismetTextLibrary.Conv_StringToText` _instrumentname))
  (`SceneComponent.SetVisibility` (`self.Description`) true false)
  (`TextRenderComponent.K2_SetText` (`self.Description`) (`KismetTextLibrary.Conv_StringToText` (`KismetTextLibrary.Conv_TextToString` _instrumentdescription)))
  (`TextRenderComponent.K2_SetText` (`self.TextRender1`) (`KismetTextLibrary.Conv_StringToText` (`KismetTextLibrary.Conv_TextToString` _instrumenthistory))))

(fn `UserConstructionScript`)